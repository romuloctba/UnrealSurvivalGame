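; Inventory actor for a survival game that stores items as class-and-amount slots and handles adding, stacking, splitting, swapping, using and discarding them.
; AddItemMaster fills partial stacks or empty slots, calling itself recursively for leftovers, and reads stack limits and weights from item class defaults.
; Using an item spawns it for OnConsume, while discarding can drop it before the player.
; Run/Trigger wrappers expose operations, and player messages update encumbrance and slot displays.
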(event Custom|UpdateInventory
  (params (InfexRef :type Integer))
  (Class|IPlayerCharacter|TriggerUpdateSlot(Message) (Game|GetPlayerCharacter 0) InfexRef))

(event EventBeginPlay
  (InventorySettings|SetNumberOfInventorySlots (Variables|InventorySettings|GetBeginingSlotAmount)))

(event EventRunSetDiscard
  (params (bDiscarded :type Boolean))
  (Variables|Bool|SetbWasDiscarded bDiscarded))

(event EventTriggerUseItem
  (params (IndexRef :type Integer))
  (InventoryItems|UseItem IndexRef))

(fn ConstructionScript)

(fn SetNumberOfInventorySlots
  (params (Size :type Integer))
  (Utilities|Array|Resize (Variables|InventorySettings|GetInventorySlotsData) Size)
  (return))

(fn AddItemMaster
  (params (ItemClass :type BP%20Item%20Master%20Class%20Reference) (Amount :type Integer))
  (LocalVariables|SetItemClassLocal ItemClass)
  (LocalVariables|SetNewAmountLocal Amount)
  (Utilities|CheckifStackable (LocalVariables|GetItemClassLocal)
    (:Stackable
      ;[1 1 1] AddStackableItem
      (LocalVariables|SetMaxStackSizeLocal (IventoryItem|GetMaxStack (LocalVariables|GetItemClassLocal)))
      (bind (_bfoundavailablestack _indexref) (SlotAvailability|FindAvailableStack (LocalVariables|GetItemClassLocal)))
      (LocalVariables|SetbStackExistsLocal _bfoundavailablestack)
      (LocalVariables|SetIndexRefLocal _indexref)
      (LocalVariables|SetcurrentStackAmountLocal (Utilities|Struct|BreakF_InventorySlot (Utilities|Array|Get(acopy) (Variables|InventorySettings|GetInventorySlotsData) (LocalVariables|GetIndexRefLocal))))
      (bind (_bhasmore _amountremaining) (UtilityFunctions|AddtoStack (LocalVariables|GetIndexRefLocal) (LocalVariables|GetItemClassLocal) (LocalVariables|GetMaxStackSizeLocal) (LocalVariables|GetNewAmountLocal) (LocalVariables|GetbStackExistsLocal)))
      (if _bhasmore
        ;;[1 1 1] Recursive call to this function
        (bind _amountremaining_2 (UtilityFunctions|AddItemMaster (LocalVariables|GetItemClassLocal) _amountremaining))
        (return true _amountremaining_2)
        (else
          (return true 0))))
    (:NonStackable
      ;[1 1 1] Finds empty slot and set index
      (bind (_bfoundemptyslot _emtyslotindex) (SlotAvailability|FindEmptySlot))
      (if _bfoundemptyslot
        (LocalVariables|SetIndexRefLocal _emtyslotindex)
        ;[1 1 1] Adds Item to inventory
        (UtilityFunctions|AddItem (LocalVariables|GetIndexRefLocal) (LocalVariables|GetItemClassLocal))
        ;[1 1 1] Encumberence System
        (Class|IPlayerCharacter|TriggerIncreaseWeight(Message) (Game|GetPlayerCharacter 0) (* 1 (UtilityFunctions|GetItemWeight (LocalVariables|GetIndexRefLocal))))
        ;[1 1 1] Check if multiple stackable items added
        (if (>= (LocalVariables|GetNewAmountLocal) 2)
          ;[1 1 1] Adjust Amount to Add
          (bind _result (Math|Integer|DecrementInt (LocalVariables|GetNewAmountLocal))
            (:%20%20
              ;[1 1 1] Recursive call to this function
              (bind _amountremaining_3 (UtilityFunctions|AddItemMaster (LocalVariables|GetItemClassLocal) _result))
              (return true _amountremaining_3)))
          (else
            (return true 0)))
        (else
          (return false (LocalVariables|GetNewAmountLocal)))))))

(fn FindEmptySlot
  (bind (_array_element _array_index) (Utilities|Array|ForEachLoopwithBreak (Variables|InventorySettings|GetInventorySlotsData) :!label _label)
    (:LoopBody
      (LocalVariables|SetInventorySlotLocal _array_element)
      (LocalVariables|SetIndexRefLocal _array_index)
      ;[1 1 1] If TRUE, slot is NOT free
      (if (Utilities|IsValidClass (.ItemClass (Utilities|Struct|BreakF_InventorySlot (LocalVariables|GetInventorySlotLocal))))
        (LocalVariables|SetIndexRefLocal -1)
        (else
          (LocalVariables|SetbIsEmptyLocal true)
          (goto _label Break))))
    (:Completed
      (return (LocalVariables|GetbIsEmptyLocal) (LocalVariables|GetIndexRefLocal)))))

(fn AddItem
  (params (Index :type Integer) (ItemClass :type BP%20Item%20Master%20Class%20Reference) (SetAmount :type Integer))
  (Utilities|Array|SetArrayElem (Variables|InventorySettings|GetInventorySlotsData) Index (Utilities|Struct|MakeF_InventorySlot ItemClass SetAmount))
  (return))

(fn GetMaxStack
  (params (Class :type BP%20Item%20Master%20Class%20Reference))
  (return (.MaxStackAmount (Utilities|Struct|BreakF_ItemDetails (.ItemDetails (Utilities|GetClassDefaults Class))))))

(fn FindAvailableStack
  (params (ItemClass :type BP%20Item%20Master%20Class%20Reference))
  (LocalVariables|SetItemClassLocal ItemClass)
  (bind (_array_element _array_index) (Utilities|Array|ForEachLoopwithBreak (Variables|InventorySettings|GetInventorySlotsData) :!label _label)
    (:LoopBody
      ;[1 1 1] 1. Is there something in the slot? 2. Is the same class (slot and pickup item) 3. is the slot < max (if yes, valid stack)
      (LocalVariables|SetInventorySlotLocal _array_element)
      (LocalVariables|SetIndexRefLocal _array_index)
      (if (Math|Boolean|ANDBoolean (Utilities|IsValidClass (.itemclass (LocalVariables|GetInventorySlotLocal))) (== (.itemclass (LocalVariables|GetInventorySlotLocal)) (LocalVariables|GetItemClassLocal)) (< (.amountinslot (LocalVariables|GetInventorySlotLocal)) (IventoryItem|GetMaxStack (LocalVariables|GetItemClassLocal))))
        (LocalVariables|SetbFoundAvailableStackLocal true)
        (goto _label Break)
        (else
          (LocalVariables|SetIndexRefLocal 0))))
    (:Completed
      (return (LocalVariables|GetbFoundAvailableStackLocal) (LocalVariables|GetIndexRefLocal)))))

(fn AddtoStack
  (params (IndexRef :type Integer) (ItemClass :type BP%20Item%20Master%20Class%20Reference) (MaxStackSize :type Integer) (AmountToAdd :type Integer) (bExistInStack :type Boolean))
  ;[1 1 1] Setting Local Variables
  (LocalVariables|SetIndexRefLocal IndexRef)
  (LocalVariables|SetItemClassLocal ItemClass)
  (LocalVariables|SetMaxStackSizeLocal MaxStackSize)
  (LocalVariables|SetAmountToAddLocal AmountToAdd)
  (LocalVariables|SetbExistInStackLocal bExistInStack)
  ;[1 1 1] TRUE: stack exists
  (if (LocalVariables|GetbExistInStackLocal)
    ;[1 1 1] Check if amount to add + current stack is less or equal than Max Stack
    (if (<= (+ (LocalVariables|GetAmountToAddLocal) (.AmountInSlot (Utilities|Struct|BreakF_InventorySlot (Utilities|Array|Get(acopy) (Variables|InventorySettings|GetInventorySlotsData) (LocalVariables|GetIndexRefLocal))))) (LocalVariables|GetMaxStackSizeLocal))
      ;[1 1 1] Add Item to existing stack
      (UtilityFunctions|AddItem (LocalVariables|GetIndexRefLocal) (LocalVariables|GetItemClassLocal) (+ (LocalVariables|GetAmountToAddLocal) (.AmountInSlot (Utilities|Struct|BreakF_InventorySlot (Utilities|Array|Get(acopy) (Variables|InventorySettings|GetInventorySlotsData) (LocalVariables|GetIndexRefLocal))))))
      ;[1 1 1] Encumberance
      (Class|IPlayerCharacter|TriggerIncreaseWeight(Message) (Game|GetPlayerCharacter 0) (* (LocalVariables|GetAmountToAddLocal) (UtilityFunctions|GetItemWeight (LocalVariables|GetIndexRefLocal))))
      (return false 0)
      (else
        ;[1 1 1] Add all items up to max amount (Both new and existing stacks use this)
        (LocalVariables|SetRemainingLocal (- (LocalVariables|GetAmountToAddLocal) (- (LocalVariables|GetMaxStackSizeLocal) (Utilities|Struct|BreakF_InventorySlot (Utilities|Array|Get(acopy) (Variables|InventorySettings|GetInventorySlotsData) (LocalVariables|GetIndexRefLocal))))) :!label _label)
        (LocalVariables|SetTempAMountLocal (- (LocalVariables|GetMaxStackSizeLocal) (Utilities|Struct|BreakF_InventorySlot (Utilities|Array|Get(acopy) (Variables|InventorySettings|GetInventorySlotsData) (LocalVariables|GetIndexRefLocal)))))
        (UtilityFunctions|AddItem (LocalVariables|GetIndexRefLocal) (LocalVariables|GetItemClassLocal) (LocalVariables|GetMaxStackSizeLocal))
        (Class|IPlayerCharacter|TriggerIncreaseWeight(Message) (Game|GetPlayerCharacter 0) (select (LocalVariables|GetbExistInStackLocal) (* (LocalVariables|GetTempAMountLocal) (UtilityFunctions|GetItemWeight (LocalVariables|GetIndexRefLocal))) (* (LocalVariables|GetMaxStackSizeLocal) (UtilityFunctions|GetItemWeight (LocalVariables|GetIndexRefLocal)))))
        (return false (LocalVariables|GetRemainingLocal))))
    (else
      ;[1 1 1] Check if Empty Slot exists
      (bind (_bfoundemptyslot _emtyslotindex) (SlotAvailability|FindEmptySlot))
      (LocalVariables|SetIndexRefLocal _emtyslotindex)
      (if _bfoundemptyslot
        ;[1 1 1] Check if Add Amount is greater than MaxStack
        (if (> (LocalVariables|GetAmountToAddLocal) (LocalVariables|GetMaxStackSizeLocal))
          (goto _label)
          (else
            ;[1 1 1] Add All Items to new Stack
            (UtilityFunctions|AddItem (LocalVariables|GetIndexRefLocal) (LocalVariables|GetItemClassLocal) (LocalVariables|GetAmountToAddLocal))
            (Class|IPlayerCharacter|TriggerIncreaseWeight(Message) (Game|GetPlayerCharacter 0) (* (LocalVariables|GetAmountToAddLocal) (UtilityFunctions|GetItemWeight (LocalVariables|GetIndexRefLocal))))
            (return false 0)))))))

(fn GetAmount
  (params (IndexRef :type Integer))
  (return (Utilities|Struct|BreakF_InventorySlot (Utilities|Array|Get(acopy) (Variables|InventorySettings|GetInventorySlotsData) IndexRef))))

(fn DiscardItem
  (params (IndexRef :type Integer) (Amount :type Integer))
  ;[1 1 1] SetLocal Variables
  (LocalVariables|SetIndexRefLocal IndexRef)
  (LocalVariables|SetAmountLocal Amount)
  ;[1 1 1] 1. Is there something in the slot? 2. Is there amount to discard
  (if (and (SlotAvailability|CheckifSlotIsFree (LocalVariables|GetIndexRefLocal)) (<= (LocalVariables|GetAmountLocal) 0))
    (return false)
    (else
      (LocalVariables|SetItemClassLocal (.itemclass (Utilities|Array|Get(acopy) (Variables|InventorySettings|GetInventorySlotsData) (LocalVariables|GetIndexRefLocal))))
      ;[1 1 1] Encumberence - Store weight of item to be discarded
      (LocalVariables|SetWeightLocal (UtilityFunctions|GetItemWeight (LocalVariables|GetIndexRefLocal)))
      ;[1 1 1] check if discard >= amount to slot
      (if (>= (LocalVariables|GetAmountLocal) (IventoryItem|GetAmount (LocalVariables|GetIndexRefLocal)))
        (UtilityFunctions|AddItem (LocalVariables|GetIndexRefLocal))
        (else
          (UtilityFunctions|AddItem (LocalVariables|GetIndexRefLocal) (.itemclass (Utilities|Array|Get(acopy) (Variables|InventorySettings|GetInventorySlotsData) (LocalVariables|GetIndexRefLocal))) (- (.amountinslot (Utilities|Array|Get(acopy) (Variables|InventorySettings|GetInventorySlotsData) (LocalVariables|GetIndexRefLocal))) (LocalVariables|GetAmountLocal)))))
      ;[1 1 1] Check if item was used or ropped
      (if (Variables|Bool|GetbWasDiscarded)
        (Game|SpawnActorfromClass (LocalVariables|GetItemClassLocal) (UtilityFunctions|SpawnTransformDiscardItem) "Undefined" 0 (Variables|Bool|GetbWasDiscarded) 0)
        (Variables|Bool|SetbWasDiscarded false))
      ;[1 1 1] Encumberance - Remover weight from player
      (Class|IPlayerCharacter|TriggerDecreaseWeight(Message) (Game|GetPlayerCharacter 0) (* (LocalVariables|GetAmountLocal) (LocalVariables|GetWeightLocal)))
      (CallFunction|UpdateInventory (LocalVariables|GetIndexRefLocal))
      (return true))))

(fn CheckifSlotIsFree
  (params (IndexRef%201 :type Integer))
  ;[1 1 1] If valid the slot is NOT free. If not valid, slot is free
  (return (not (Utilities|IsValidClass (.ItemClass (Utilities|Struct|BreakF_InventorySlot (Utilities|Array|Get(acopy) (Variables|InventorySettings|GetInventorySlotsData) IndexRef%201)))))))

(fn SpawnTransformDiscardItem
  (bind _returnvalue (Game|GetPlayerCharacter 0))
  (bind _returnvalue_2 (Transformation|GetActorTransform _returnvalue))
  (return (Math|Transform|MakeTransform (+ (* (Transformation|GetActorForwardVector _returnvalue) 3e+02) (.location _returnvalue_2)) (.rotation _returnvalue_2) (.scale _returnvalue_2))))

(fn ChangeSlots
  (params (IndexRefA :type Integer) (IndexRefB :type Integer))
  (bind _inventoryslotsdata (Variables|InventorySettings|GetInventorySlotsData))
  (bind _inventoryslotsdata_2 (Variables|InventorySettings|GetInventorySlotsData))
  (bind _returnvalue (Utilities|Array|LastIndex _inventoryslotsdata))
  ;[1 1 1] set local slots that are swapping
  (LocalVariables|SetIndexRefALocal IndexRefA)
  (LocalVariables|SetIndexRefBLocal IndexRefB)
  ;[1 1 1] Check inventory bounds. TRUE = out of bounds
  (if (or (> (LocalVariables|GetIndexRefALocal) _returnvalue) (> (LocalVariables|GetIndexRefBLocal) _returnvalue))
    (return false)
    (else
      ;[1 1 1] Dtore item in slot b in temp variable. b will be overriden by A
      (LocalVariables|SetTempHoldingLocal (Utilities|Array|Get(acopy) (Variables|InventorySettings|GetInventorySlotsData) (LocalVariables|GetIndexRefBLocal)))
      ;[1 1 1] Override item in B with item in A
      (Utilities|Array|SetArrayElem _inventoryslotsdata_2 (LocalVariables|GetIndexRefBLocal) (Utilities|Array|Get(acopy) _inventoryslotsdata_2 (LocalVariables|GetIndexRefALocal)))
      ;[1 1 1] "Restore"(from temp) B in A former slot
      (Utilities|Array|SetArrayElem (Variables|InventorySettings|GetInventorySlotsData) (LocalVariables|GetIndexRefALocal) (LocalVariables|GetTempHoldingLocal))
      (CallFunction|UpdateInventory (LocalVariables|GetIndexRefALocal))
      (CallFunction|UpdateInventory (LocalVariables|GetIndexRefBLocal))
      (return true))))

(fn SplitStack
  (params (IndexRef :type Integer) (SplitAmount :type Integer))
  ;[1 1 1] Set Local Variables
  (LocalVariables|SetIndexRefLocal IndexRef)
  (LocalVariables|SetSplitAmountLocal SplitAmount)
  ;[1 1 1] Is Slot Free?
  (if (SlotAvailability|CheckifSlotIsFree (LocalVariables|GetIndexRefLocal))
    (return false)
    (else
      ;[1 1 1] 1. NOT oversplitting 2. is harvestable
      (if (and (Utilities|Struct|BreakF_ItemDetails (.Item%20Details (IventoryItem|GetItemInfo (LocalVariables|GetIndexRefLocal)))) (> (.Amount%20in%20Slot (IventoryItem|GetItemInfo (LocalVariables|GetIndexRefLocal))) (LocalVariables|GetSplitAmountLocal)))
        ;[1 1 1] Find New Slot
        (bind (_bfoundemptyslot _emtyslotindex) (SlotAvailability|FindEmptySlot))
        (if _bfoundemptyslot
          (LocalVariables|SetNewIndexRefLocal _emtyslotindex)
          ;[1 1 1] Adjust the original Stack
          (UtilityFunctions|AddItem (LocalVariables|GetIndexRefLocal) (.itemclass (Utilities|Array|Get(acopy) (Variables|InventorySettings|GetInventorySlotsData) (LocalVariables|GetIndexRefLocal))) (- (.amountinslot (Utilities|Array|Get(acopy) (Variables|InventorySettings|GetInventorySlotsData) (LocalVariables|GetIndexRefLocal))) (LocalVariables|GetSplitAmountLocal)))
          ;[1 1 1] Add new Stack
          (UtilityFunctions|AddItem (LocalVariables|GetNewIndexRefLocal) (.itemclass (Utilities|Array|Get(acopy) (Variables|InventorySettings|GetInventorySlotsData) (LocalVariables|GetIndexRefLocal))) (LocalVariables|GetSplitAmountLocal))
          (CallFunction|UpdateInventory (LocalVariables|GetIndexRefLocal))
          (CallFunction|UpdateInventory (LocalVariables|GetNewIndexRefLocal))
          (Class|IPlayerCharacter|TriggerSetupInventorySlots(Message) (Game|GetPlayerCharacter 0))
          (return true)
          (else
            (return false)))
        (else
          (return false))))))

(fn GetItemInfo
  (params (IndexRef :type Integer))
  (bind _inventoryslotsdata (Variables|InventorySettings|GetInventorySlotsData))
  (bind _output (Utilities|Array|Get(acopy) _inventoryslotsdata IndexRef))
  (bind _returnvalue (Utilities|IsValidClass (.itemclass _output)))
  ;[1 1 1] Confirm Slot is Empty
  (LocalVariables|SetbIsEmptyLocal (not _returnvalue))
  ;[1 1 1] CheckSlot is Filled
  (if _returnvalue
    (return (LocalVariables|GetbIsEmptyLocal) (.ItemDetails (Utilities|GetClassDefaults (.itemclass _output))) (.amountinslot _output))
    (else
      (return (LocalVariables|GetbIsEmptyLocal) "" 0))))

(fn UseItem
  (params (IndexRef :type Integer))
  (LocalVariables|SetIndexRefLocal IndexRef)
  (if (Utilities|IsValidClass (.ItemClass (Utilities|Struct|BreakF_InventorySlot (Utilities|Array|Get(acopy) (Variables|InventorySettings|GetInventorySlotsData) (LocalVariables|GetIndexRefLocal)))))
    (bind _returnvalue (Game|SpawnActorfromClass (.ItemClass (Utilities|Struct|BreakF_InventorySlot (Utilities|Array|Get(acopy) (Variables|InventorySettings|GetInventorySlotsData) (LocalVariables|GetIndexRefLocal)))) (LocalVariables|GetEmptyTransformLocal) "AlwaysSpawn" 0 false 0))
    (Default|OnConsume _returnvalue (LocalVariables|GetIndexRefLocal))
    (return)))

(fn GetItemWeight
  (params (IndexRef%201 :type Integer))
  (return (Utilities|Struct|BreakF_ItemDetails (Utilities|GetClassDefaults (.itemclass (Utilities|Array|Get(acopy) (Variables|InventorySettings|GetInventorySlotsData) IndexRef%201))))))

(fn GetInventoryActorReference
  (return self))

(fn GetSlotsData
  (return (Variables|InventorySettings|GetInventorySlotsData)))

(fn RunCheckifSlotIsFree
  (params (IndexRef :type Integer))
  (return (SlotAvailability|CheckifSlotIsFree IndexRef)))

(fn RunDiscardItem
  (params (IndexRef :type Integer) (Amount :type Integer))
  (bind _bitemremoved (UtilityFunctions|DiscardItem IndexRef Amount))
  (return _bitemremoved))

(fn RunGetItemInfo
  (params (IndexRef :type Integer))
  (bind (_bisemty _item_details _amount_in_slot) (IventoryItem|GetItemInfo IndexRef))
  (return _bisemty _item_details _amount_in_slot))

(fn RunSplitStack
  (params (IndexRef :type Integer) (SplitAmount :type Integer))
  (bind _bsplitsucessful (UtilityFunctions|SplitStack IndexRef SplitAmount))
  (return _bsplitsucessful))

(fn TriggerAddItemMaster
  (params (ItemClass :type BP%20Item%20Master%20Class%20Reference) (ItemAmount :type Integer))
  (bind (_bsuccessfullyadded _amountremaining) (UtilityFunctions|AddItemMaster ItemClass ItemAmount))
  (return _bsuccessfullyadded _amountremaining))