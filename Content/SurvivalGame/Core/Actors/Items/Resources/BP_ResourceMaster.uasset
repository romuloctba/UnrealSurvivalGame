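; BP_ResourceMaster is the base resource item actor, which sets how much of a resource each instance holds.
; Its construction script runs the parent's, then, for spawned instances that were not discarded, derives ItemAmount from the rounded product of BaseAmount and the mesh's world scale on all three axes.
; Amount therefore scales with the mesh's volume, and the event graph holds only disabled stub events.
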(event EventBeginPlay
  (|CallParentFunction) ; This node is disabled and will not be called.\nDrag off pins to build functionality.
)

(event Collision|EventActorBeginOverlap
  (params (OtherActor :type Actor%20Object%20Reference))
  (|CallParentFunction OtherActor) ; This node is disabled and will not be called.\nDrag off pins to build functionality.
)

(event EventTick
  (params (DeltaSeconds :type Float%20%28single-precision%29))
  (|CallParentFunction DeltaSeconds) ; This node is disabled and will not be called.\nDrag off pins to build functionality.
)

(fn ConstructionScript
  (bind _itemmesh (Variables|Default|GetItemMesh))
  (bind _returnvalue (Transformation|GetWorldScale _itemmesh))
  (bind (_x _y _z) (Math|Vector|BreakVector _returnvalue))
  (|CallParentFunction)
  (if (not (Variables|Default|GetbWasDiscarded))
    (if (Variables|Bools|GetbWasSpawn)
      (Variables|Default|SetItemAmount (Math|Float|Round (* (Variables|WorldSettings|GetBaseAmount) (* _x _y _z)))))))