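; Base world item actor for the survival game, picked up by the player, with an overridable OnConsume hook.
; Construction fits the trigger box to the mesh, or enables physics for discarded items.
; Player overlap, gated by a busy flag and camera trace for any WorldDynamic hit, shows a harvest prompt or picks up immediately.
; Pickup messages the inventory, keeping any remainder or retriggering player overlap and destroying the actor.
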(event OnComponentBeginOverlap(Box)
  (params (OverlappedComponent :type Primitive%20Component%20Object%20Reference) (OtherActor :type Actor%20Object%20Reference) (OtherComp :type Primitive%20Component%20Object%20Reference) (OtherBodyIndex :type Integer) (bFromSweep :type Boolean) (SweepResult :type Hit%20Result%20Structure%20%28by%20ref%29))
  ;[1 1 1] Confirms Player
  (if (== OtherActor (Game|GetPlayerCharacter 0))
    ;[1 1 1] CONFIRMS player is not already in overlap event
    (bind _bisoverlapping (Class|IPlayerCharacter|GetIsOverlapping(Message) OtherActor))
    (if (not _bisoverlapping)
      ;[1 1 1] Checks if player is looking at item
      (bind _bplayerseesitem (CallFunction|CheckifPlayerSeesItem))
      (if _bplayerseesitem
        ;[1 1 1] Set and Determine if player is Overlapping
        (Class|IPlayerCharacter|ISetIsOverlapping(Message) OtherActor true)
        (bind _bisoverlapping_2 (Class|IPlayerCharacter|GetIsOverlapping(Message) OtherActor))
        (if _bisoverlapping_2
          (CallFunction|OverlapTrigger))))))

(event OnComponentEndOverlap(Box)
  (params (OverlappedComponent :type Primitive%20Component%20Object%20Reference) (OtherActor :type Actor%20Object%20Reference) (OtherComp :type Primitive%20Component%20Object%20Reference) (OtherBodyIndex :type Integer))
  (bind _returnvalue (Game|GetPlayerCharacter 0))
  ;[1 1 1] Player no longer overlap && item is harvestable
  (bind _bisoverlapping (Class|IPlayerCharacter|GetIsOverlapping(Message) OtherActor))
  (if (and _bisoverlapping (Utilities|Struct|BreakF_ItemDetails (Variables|Master|GetItemDetails)))
    (Class|IPlayerCharacter|EndHarvestPromp(Message) _returnvalue)
    (Class|IPlayerCharacter|ISetIsOverlapping(Message) _returnvalue false)))

(event Custom|OverlapTrigger
  ;[1 1 1] Pickup event or Prompt to pikupt event
  (if (Utilities|Struct|BreakF_ItemDetails (Variables|Master|GetItemDetails))
    (Class|IPlayerCharacter|TriggerHarverstPrompt(Message) (Game|GetPlayerCharacter 0) self (Variables|Master|GetItemDetails))
    (else
      (CallFunction|TriggerPickupObject))))

(event Custom|OnConsume
  (params (IndexRef :type Integer))
  ;[1 1 1] Override Consumer Event
)

(event Custom|AbortOverlap
  (bind _returnvalue (Game|GetPlayerCharacter 0))
  (Class|IPlayerCharacter|EndHarvestPromp(Message) _returnvalue)
  (Class|IPlayerCharacter|ISetIsOverlapping(Message) _returnvalue false))

(event EventBeginPlay
  (if (not (>= (Variables|WorldSettings|GetItemAmount) 1))
    (Actor|DestroyActor)))

(event Collision|EventActorBeginOverlap
  (params (OtherActor :type Actor%20Object%20Reference)))

(event EventTick
  (params (DeltaSeconds :type Float%20%28single-precision%29)))

(event EventTriggerPickupObject
  (bind _returnvalue (Game|GetPlayerCharacter 0))
  ;[1 1 1] Pickup event and retrigger prompt if needed
  (if (>= (Variables|WorldSettings|GetItemAmount) 1)
    (bind _bactortobedestroyed (CallFunction|PickUpObject (Variables|WorldSettings|GetItemAmount)))
    (if _bactortobedestroyed
      (Class|IPlayerCharacter|PlayerRetriggerOverlap(Message) _returnvalue self)
      (Actor|DestroyActor)
      (Class|IPlayerCharacter|ISetIsOverlapping(Message) _returnvalue false))
    (else
      (Class|IPlayerCharacter|ISetIsOverlapping(Message) (Game|GetPlayerCharacter 0) false)
      (CallFunction|AbortOverlap))))

(event EventItemRetriggerOverlap
  ;[1 1 1] Set and Determine if player is Overlapping
  (Class|IPlayerCharacter|ISetIsOverlapping(Message) (stale OnComponentBeginOverlap(Box) OtherActor) true)
  (bind _bisoverlapping (Class|IPlayerCharacter|GetIsOverlapping(Message) (stale OnComponentBeginOverlap(Box) OtherActor)))
  (if _bisoverlapping
    (CallFunction|OverlapTrigger)))

(fn ConstructionScript
  (bind _box (Variables|Default|GetBox))
  (bind _itemmesh (Variables|Default|GetItemMesh))
  (bind _customcollisionsize (Variables|Master|GetCustomCollisionSize))
  (bind _itemmesh_2 (Variables|Default|GetItemMesh))
  (bind _max (Components|StaticMesh|GetLocalBounds _itemmesh))
  (bind _returnvalue (* _max _customcollisionsize))
  (if (not (Variables|bool|GetbWasDiscarded))
    (Components|Box|SetBoxExtent _box _returnvalue true)
    (if (Variables|bool|GetbAdjustColisionOffset)
      (Transformation|AddLocalOffset _box (Math|Vector|MakeVector 0.0 0.0 (.Z (Math|Vector|BreakVector _returnvalue))) false true))
    (else
      (Physics|SetSimulatePhysics _itemmesh_2 true)
      (Physics|SetEnableGravity _itemmesh_2 true)
      (Collision|SetCollisionProfileName _itemmesh_2 "BlockAllDynamic" true :!class /Script/Engine.PrimitiveComponent))))

(fn PickUpObject
  (params (AmountToAdd :type Integer))
  (bind _inventoryactor (Class|IPlayerCharacter|IGetInventoryActor(Message) (Game|GetPlayerCharacter 0)))
  (Utilities|IsValid _inventoryactor
    (:Is%20Valid
      (bind _amountremaining (Class|IInventory|TriggerAddItemMaster(Message) _inventoryactor (Variables|Master|GetItemClass) AmountToAdd))
      (if true
        (if (select (== AmountToAdd (Variables|WorldSettings|GetItemAmount)) (>= _amountremaining 1) (>= (- (Variables|WorldSettings|GetItemAmount) AmountToAdd) 1))
          (Variables|WorldSettings|SetItemAmount (select (== AmountToAdd (Variables|WorldSettings|GetItemAmount)) _amountremaining (+ _amountremaining (- (Variables|WorldSettings|GetItemAmount) AmountToAdd))))
          (return false)
          (else
            (return true)))))))

(fn CheckifPlayerSeesItem
  (bind _returnvalue (Game|GetPlayerCameraManager 0))
  (bind _returnvalue_2 (Transformation|GetActorLocation _returnvalue))
  (bind _returnvalue_3 (Transformation|GetActorForwardVector _returnvalue))
  (bind _returnvalue_4 (Class|KismetSystemLibrary|LineTraceMultiforObjects (+ _returnvalue_2 (* _returnvalue_3 15.0)) (+ _returnvalue_2 (* _returnvalue_3 5e+02)) (Utilities|Array|MakeArray "ObjectTypeQuery2") false (Utilities|Array|MakeArray (Game|GetPlayerCharacter 0)) "None" false "(R=1.000000,G=0.000000,B=0.000000,A=1.000000)" "(R=0.000000,G=1.000000,B=0.000000,A=1.000000)" 1e+01))
  (return _returnvalue_4))